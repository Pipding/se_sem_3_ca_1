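; Securibot enemy character that kills the player on contact with its kill capsule, then quits the game after a caught bark.
; Spotting the player turns its material eyes and spotlights red and notifies the first-person character.
; Tick feeds movement and turn direction, derived from velocity and desired controller rotation, to ABP_Securibot.
; Voice barks fire as triggers on a manually spawned, attached MetaSound, with a timer tracking time since the last chase bark.
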(event `self.ReceiveBeginPlay`
  ;[1 1 1] Create a dynamic material so we can change eye colour at runtime
  (bind _returnvalue (`PrimitiveComponent.CreateDynamicMaterialInstance` (`self.Mesh`) 0 "/Game/Assets/Materials/M_Securibot.M_Securibot" "None"))
  (set `self.MeshMaterial` _returnvalue)
  (`self.SetEyeColour` (struct :`R` 0.047059 :`G` 0.117647 :`B` 0.772549 :`A` 1.0))
  ;[1 1 1] For some unknowable reason, custom triggers only work if we spawn the metasound and attach it manually
  (bind _returnvalue_2 (`GameplayStatics.SpawnSoundAttached` "/Game/Assets/Audio/VO/Securibot/MS_Securibot.MS_Securibot" (`self.CapsuleComponent`) "None" (0.0 0.0 0.0) (struct) "KeepRelativeOffset" false 1.0 1.0 0.0 null null))
  (set `self.MS_Securibot` _returnvalue_2))

(event `SetCanSeePlayer`
  (params (NewValue :type Boolean))
  (bind _asabp_securibot (cast `/Game/Characters/Securibot/ABP_Securibot` (`SkeletalMeshComponent.GetAnimInstance` (`self.Mesh`))))
  (bind _output_get (set `/Game/Characters/Securibot/ABP_Securibot.CanSeePlayer` NewValue _asabp_securibot))
  (if _output_get
    (`self.SetEyeColour` (struct :`R` 1.0 :`G` 0.09375 :`B` 0.107935 :`A` 1.0))
    (bind _asbp_first_person_character (cast `/Game/Blueprints/BP_FirstPersonCharacter` (`GameplayStatics.GetPlayerCharacter` 0)))
    (`/Game/Blueprints/BP_FirstPersonCharacter.SpottedBySecuribotEvent` _asbp_first_person_character)
    (else
      (`self.SetEyeColour` (struct :`R` 0.047059 :`G` 0.117647 :`B` 0.772549 :`A` 1.0)))))

(event `self.CapsuleComponentKill.OnComponentBeginOverlap`
  (params (OverlappedComponent :type "PrimitiveComponent Object Reference") (OtherActor :type "Actor Object Reference") (OtherComp :type "PrimitiveComponent Object Reference") (OtherBodyIndex :type Integer) (bFromSweep :type Boolean) (SweepResult :type "HitResult Structure (by ref)"))
  (bind _asbp_first_person_character (cast `/Game/Blueprints/BP_FirstPersonCharacter` OtherActor))
  (`/Game/Blueprints/BP_FirstPersonCharacter.SetIsAlive` _asbp_first_person_character false)
  (set `self.CanDetectPlayer` false)
  (`KismetSystemLibrary.Delay` 0.75)
  (`self.Bark_CaughtPlayer`)
  (`KismetSystemLibrary.Delay` 3.0)
  (`KismetSystemLibrary.QuitGame` null "Quit"))

(event `self.ReceiveTick`
  (params (DeltaSeconds :type "Float (single-precision)"))
  (`|ExecutionSequence`
    (:`then_0`
      (`self.UpdateChasingBarkTimer` DeltaSeconds))
    (:`then_1`
      ;[1 1 1] Check if robot is rotating
      (bind _returnvalue (`self.RotationMatchesTargetRotation`))
      (`self.SetIsRotating` (not _returnvalue)))
    (:`then_2`
      ;[1 1 1] Check if robot is moving
      (`self.IsWalkingOnGround`
        (:`yes`
          (set `self.IsMoving` true))
        (:`no`
          (set `self.IsMoving` false)))
      (bind _asabp_securibot (cast `/Game/Characters/Securibot/ABP_Securibot` (`SkeletalMeshComponent.GetAnimInstance` (`self.Mesh`))))
      (set `/Game/Characters/Securibot/ABP_Securibot.IsMoving` (`self.IsMoving`) _asabp_securibot))))

(fn `Bark_CaughtPlayer`
  (message `AudioParameterControllerInterface.SetTriggerParameter` (`self.MS_Securibot`) "PlayCaughtPlayer"))

(fn `Bark_ChaseInitiated`
  (message `AudioParameterControllerInterface.SetTriggerParameter` (`self.MS_Securibot`) "PlaySeesPlayer"))

(fn `Bark_ChasingPlayer`
  (message `AudioParameterControllerInterface.SetTriggerParameter` (`self.MS_Securibot`) "PlayIsChasing")
  (set `self.Bark_Chase_TimeSinceLastBark` 0.0))

(fn `Bark_LostPlayer`
  (message `AudioParameterControllerInterface.SetTriggerParameter` (`self.MS_Securibot`) "PlayLostPlayer"))

(fn `Bark_ReturnToPatrol`
  (message `AudioParameterControllerInterface.SetTriggerParameter` (`self.MS_Securibot`) "PlayReturnToPatrol"))

(fn `PlayWarning`
  (message `AudioParameterControllerInterface.SetTriggerParameter` (`self.MS_Securibot`) "PlayWarning"))

(fn `RotationMatchesTargetRotation`
  (returns (ReturnValue :type Boolean))
  (return (== (`Controller.GetDesiredRotation` (`self.GetController`)) (`SceneComponent.K2_GetComponentRotation` (`self.CapsuleComponent`)) :`ErrorTolerance` 0.1)))

(fn `SetEyeColour`
  (params (Value :type "LinearColor Structure"))
  (`MaterialInstanceDynamic.SetVectorParameterValue` (`self.MeshMaterial`) "EyeColour" Value)
  (`PrimitiveComponent.SetMaterial` (`self.Mesh`) 0 (`self.MeshMaterial`))
  (`LightComponent.SetLightColor` (`self.SpotlightEyeR`) Value true)
  (`LightComponent.SetLightColor` (`self.SpotlightEyeL`) Value true))

(fn `SetIsRotating`
  (params (IsRotating :type Boolean))
  (locals (SecuribotAnim :type "/Game/Characters/Securibot/ABP_Securibot Object Reference"))
  (bind _securibotanim (`local.SecuribotAnim`))
  (bind _securibotanim_2 (`local.SecuribotAnim`))
  (bind _securibotanim_3 (`local.SecuribotAnim`))
  (bind _asabp_securibot (cast `/Game/Characters/Securibot/ABP_Securibot` (`SkeletalMeshComponent.GetAnimInstance` (`self.Mesh`))))
  (set `local.SecuribotAnim` _asabp_securibot)
  (bind _output_get (set `self.IsRotating` IsRotating))
  (if _output_get
    (`self.IsRotatingWhichDirection`
      (:`Right`
        (set `self.IsRotatingLeft` false)
        (set `self.IsRotatingRight` true)
        (set `/Game/Characters/Securibot/ABP_Securibot.IsRotatingL` false _securibotanim_3)
        (set `/Game/Characters/Securibot/ABP_Securibot.IsRotatingR` true _securibotanim_3)
        (set `/Game/Characters/Securibot/ABP_Securibot.IsRotating` true _securibotanim_3))
      (:`Left`
        (set `self.IsRotatingLeft` true)
        (set `self.IsRotatingRight` false)
        (set `/Game/Characters/Securibot/ABP_Securibot.IsRotatingL` true _securibotanim_2)
        (set `/Game/Characters/Securibot/ABP_Securibot.IsRotatingR` false _securibotanim_2)
        (set `/Game/Characters/Securibot/ABP_Securibot.IsRotating` true _securibotanim_2)))
    (else
      (set `self.IsRotatingLeft` false)
      (set `self.IsRotatingRight` false)
      (set `/Game/Characters/Securibot/ABP_Securibot.IsRotatingL` false _securibotanim)
      (set `/Game/Characters/Securibot/ABP_Securibot.IsRotatingR` false _securibotanim)
      (set `/Game/Characters/Securibot/ABP_Securibot.IsRotating` false _securibotanim))))

(fn `UpdateChasingBarkTimer`
  (params (DeltaTime :type "Float (double-precision)"))
  (returns (TimeSinceLastBark :type "Float (double-precision)"))
  (if (`self.IsChasingPlayer`)
    (bind _output_get (set `self.Bark_Chase_TimeSinceLastBark` (+ DeltaTime (`self.Bark_Chase_TimeSinceLastBark`))))
    (return _output_get)))

(fn `UserConstructionScript`)