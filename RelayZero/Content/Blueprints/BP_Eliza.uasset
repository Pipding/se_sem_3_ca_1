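; BP_Eliza is an interactable actor that the player can wake to play a chime and report a noise at its location.
; Quick interact fires the chime directly, while the interaction menu, a WeaponWheel widget created on BeginPlay, offers a single Wake segment that fires it on close if selected.
; An outline glow event sets custom depth and stencil on its Cone component, logic noted as duplicated across other interface implementations.
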(event `self.ReceiveBeginPlay`
  (bind _returnvalue (`|CreateWidget` "/Game/UI/WeaponWheel/WeaponWheel.WeaponWheel_C"))
  (set `self.InteractionMenu` _returnvalue))

(event `/Game/Interfaces/BPI_Interactable.OnPlayerQuickInteract`
  ;[1 1 1] Quick interaction (E key)
  (`self.PlayWakeChimeEvent`))

(event `/Game/Interfaces/BPI_Interactable.OnPlayerOpenInteractMenu`
  ;[1 1 1] Interaction menu (Q key)
  (`/Game/UI/WeaponWheel/WeaponWheel.OpenMenu` (`self.InteractionMenu`))
  (`self.SetUpInteractionMenu`))

(event `/Game/Interfaces/BPI_Interactable.OnPlayerCloseInteractMenu`
  ;[1 1 1] Interaction menu (Q key)
  (`self.HandleInteractionMenuSelection`)
  (`/Game/UI/WeaponWheel/WeaponWheel.CloseMenu` (`self.InteractionMenu`)))

(event `PlayWakeChimeEvent`
  (bind _returnvalue (`self.K2_GetActorLocation`))
  (`GameplayStatics.PlaySoundAtLocation` "/Game/Sound/FX/wake_chime.wake_chime" _returnvalue (struct) 1.0 1.0 0.0 null null null null)
  (`AISense_Hearing.ReportNoiseEvent` _returnvalue 1.0 self 1500.0))

(event `/Game/Interfaces/BPI_OutlineGlow.SetOutlineGlow`
  (params (Enabled :type Boolean) (OutlineType :type "/Game/Enums/E_PostProcessingOutlineChannel Enum" :default "NewEnumerator0"))
  (bind _cone (`self.Cone`))
  ;[1 1 1] TODO: This functionality is duplicated across all implementations. See if it can be defined in the interface
  (`PrimitiveComponent.SetRenderCustomDepth` _cone Enabled)
  (`PrimitiveComponent.SetCustomDepthStencilValue` _cone (`KismetMathLibrary.Conv_ByteToInt` OutlineType)))

(event `TestEvent_TriggerChime`
  (`self.PlayWakeChimeEvent`))

(fn `HandleInteractionMenuSelection`
  (bind _value (`/Game/UI/WeaponWheel/WeaponWheel.GetSelectedSegmentText` (`self.InteractionMenu`)))
  (switch `string` _value
    (:`Wake`
      (`self.PlayWakeChimeEvent`))))

(fn `UserConstructionScript`)