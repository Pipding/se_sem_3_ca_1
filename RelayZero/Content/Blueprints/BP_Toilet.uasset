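; BP_Toilet is an interactable toilet that the player can flush by quick interact or through a directional interaction menu.
; Flushing plays FlushAudio and holds IsFlushing for the length of the sound, blocking quick interact and menu opening meanwhile.
; The menu offers Flush in its north segment, and its selection is handled on close.
; Outline highlighting uses the mesh's custom depth stencil and is forced off during a flush.
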(event `/Game/Interfaces/BPI_OutlineGlow.SetOutlineGlow`
  (params (Enabled :type Boolean) (OutlineType :type "/Game/Enums/E_PostProcessingOutlineChannel Enum" :default "NewEnumerator0"))
  (bind _toiletmesh (`self.ToiletMesh`))
  (bind _toiletmesh_2 (`self.ToiletMesh`))
  (if (`self.IsFlushing`)
    (`PrimitiveComponent.SetRenderCustomDepth` _toiletmesh_2 false)
    (`PrimitiveComponent.SetCustomDepthStencilValue` _toiletmesh_2 0)
    (else
      (`PrimitiveComponent.SetRenderCustomDepth` _toiletmesh Enabled)
      (`PrimitiveComponent.SetCustomDepthStencilValue` _toiletmesh (`KismetMathLibrary.Conv_ByteToInt` OutlineType)))))

(event `/Game/Interfaces/BPI_Interactable.OnPlayerQuickInteract`
  (if (not (`self.IsFlushing`))
    (`self.FlushEvent`)))

(event `/Game/Interfaces/BPI_Interactable.OnPlayerOpenInteractMenu`
  ;[1 1 1] Interaction menu
  (if (not (`self.IsFlushing`))
    (`/Game/UI/WeaponWheel/WeaponWheel.OpenMenu` (`self.InteractionMenu`))
    (`self.UpdateInteractionMenu`)))

(event `/Game/Interfaces/BPI_Interactable.OnPlayerCloseInteractMenu`
  ;[1 1 1] Interaction menu
  (`self.HandleInteractionMenuSelection`)
  (`/Game/UI/WeaponWheel/WeaponWheel.CloseMenu` (`self.InteractionMenu`)))

(event `FlushEvent`
  (`self.Flush`))

(fn `HandleInteractionMenuSelection`
  (bind _value (`/Game/UI/WeaponWheel/WeaponWheel.GetSelectedSegmentText` (`self.InteractionMenu`)))
  (switch `string` _value
    (:`Flush`
      (`self.FlushEvent`))))

(fn `UpdateInteractionMenu`
  (if (`self.IsFlushing`)
    (`self.UpdateInteractionMenuFlushing`)
    (else
      (`self.UpdateInteractionMenuFlushable`))))

(fn `UserConstructionScript`)