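; BP_BurglarAlarm is an interactable burglar alarm that the player can disable to activate its controlled doors.
; Quick interact, or the Disable segment of its radial interaction menu, calls DisableAlarmEvent while the alarm is enabled.
; That event sets each linked door active, clears IsEnabled and records a Quinn voice line in the GameInstance.
; An outline glow uses custom depth stencil on the cube and is only shown while enabled.
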(event `/Game/Interfaces/BPI_OutlineGlow.SetOutlineGlow`
  (params (Enabled :type Boolean) (OutlineType :type "/Game/Enums/E_PostProcessingOutlineChannel Enum" :default "NewEnumerator0"))
  (bind _cube (`self.Cube`))
  ;[0.7452 0.5103 1] Make outline glow
  (if (`self.IsEnabled`)
    (`PrimitiveComponent.SetRenderCustomDepth` _cube Enabled)
    (`PrimitiveComponent.SetCustomDepthStencilValue` _cube (`KismetMathLibrary.Conv_ByteToInt` OutlineType))
    (else
      (`PrimitiveComponent.SetRenderCustomDepth` (`self.Cube`) false) ; Disable outline glow
    )))

(event `/Game/Interfaces/BPI_Interactable.OnPlayerQuickInteract`
  ;[0.2532 0.2549 1] Interaction
  ;;[1 1 1] Quick interact
  (if (`self.IsEnabled`)
    (`self.DisableAlarmEvent`)))

(event `/Game/Interfaces/BPI_Interactable.OnPlayerOpenInteractMenu`
  ;[0.2532 0.2549 1] Interaction
  ;;[1 1 1] Interaction menu
  (if (`self.IsEnabled`)
    (`/Game/UI/WeaponWheel/WeaponWheel.OpenMenu` (`self.InteractionMenu`))
    (`self.UpdateInteractionMenu`)))

(event `/Game/Interfaces/BPI_Interactable.OnPlayerCloseInteractMenu`
  ;[0.2532 0.2549 1] Interaction
  ;;[1 1 1] Interaction menu
  (if (`self.IsEnabled`)
    (`self.HandleInteractionMenuSelection`)
    (`/Game/UI/WeaponWheel/WeaponWheel.CloseMenu` (`self.InteractionMenu`))))

(event `DisableAlarmEvent`
  ;[0.5365 0.5365 0.5365] Disable alarm
  (for _array_element (`self.ControlledDoors`)
    (set `/Game/Blueprints/BP_DoorDouble.IsActive` true _array_element)
    (set `self.IsEnabled` false)
    (bind _asbp_relay_zero_game_instance (`/Game/Blueprints/FunctionLibraries/BML_Utils.GetGameInstance`))
    (`BlueprintMapLibrary.Map_Add` (`/Game/FirstPerson/Blueprints/BP_RelayZeroGameInstance.VoiceLinesPlayedQuinn` _asbp_relay_zero_game_instance) "quinn_audio_002" true)))

(fn `HandleInteractionMenuSelection`
  (bind _value (`/Game/UI/WeaponWheel/WeaponWheel.GetSelectedSegmentText` (`self.InteractionMenu`)))
  (switch `string` _value
    (:`Disable`
      (`self.DisableAlarmEvent`))))

(fn `UpdateInteractionMenu`
  (if (`self.IsEnabled`)
    (`self.UpdateInteractionMenuEnabled` (`self.InteractionMenu`))
    (else
      (`self.UpdateInteractionMenuDisabled` (`self.InteractionMenu`)))))

(fn `UserConstructionScript`)