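; BP_Objective is a computer objective that the player must keep in sight for a time limit to complete, unlocking the level exit.
; Quick interact starts a Tick-driven timer, and a camera-to-computer line trace interrupts it when something else blocks the view.
; Completion notifies the game instance, so overlapping the end trigger then quits the game after a delay.
; Custom depth stencil drives the computer's outline glow, and state changes are forwarded to the player character.
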(event `self.ReceiveBeginPlay`
  (add `self.OnActorBeginOverlap` (`self.EndLevelTrigger`) (delegate `LevelEndTriggerOverlapped`))
  (bind _asbp_first_person_character (cast `/Game/Blueprints/BP_FirstPersonCharacter` (`GameplayStatics.GetPlayerPawn` 0)))
  (set `self.PlayerCharacter` _asbp_first_person_character))

(event `LevelEndTriggerOverlapped` :!signature `self.OnActorBeginOverlap`
  (params (OverlappedActor :type "Actor Object Reference") (OtherActor :type "Actor Object Reference"))
  (cast `/Game/Blueprints/BP_FirstPersonCharacter` OtherActor)
  (if (`self.Completed`)
    (`KismetSystemLibrary.PrintString` "Level complete")
    (`KismetSystemLibrary.Delay` 3.0)
    (`KismetSystemLibrary.QuitGame` null "Quit")))

(event `self.ReceiveTick`
  (params (DeltaSeconds :type "Float (single-precision)"))
  (`self.IncrementTimer` DeltaSeconds (`self.TimerEnabled`)
    (:`Continue`
      (`self.CanPlayerSeeObjective`)
      (`KismetSystemLibrary.PrintString` (`KismetStringLibrary.Conv_DoubleToString` (`self.Timer`)) true true (struct :`G` 0.66 :`B` 1.0 :`A` 1.0) DeltaSeconds))
    (:`TimeUp`
      (`self.ObjectiveCompletedEvent`))))

(event `/Game/Interfaces/BPI_OutlineGlow.SetOutlineGlow`
  (params (Enabled :type Boolean) (OutlineType :type "/Game/Enums/E_PostProcessingOutlineChannel Enum" :default "NewEnumerator0"))
  (bind _sm_computer01 (`self.SM_Computer01`))
  (`PrimitiveComponent.SetRenderCustomDepth` _sm_computer01 Enabled)
  (`PrimitiveComponent.SetCustomDepthStencilValue` _sm_computer01 (`KismetMathLibrary.Conv_ByteToInt` OutlineType))
  (`/Game/Blueprints/BP_FirstPersonCharacter.ObjectiveSpottedEvent` (`self.PlayerCharacter`)))

(event `/Game/Interfaces/BPI_Interactable.OnPlayerQuickInteract`
  (`self.ObjectiveActivatedEvent`))

(event `ObjectiveActivatedEvent`
  (set `self.TimerEnabled` true)
  (`/Game/Blueprints/BP_FirstPersonCharacter.ObjectiveActivatedEvent` (`self.PlayerCharacter`)))

(event `ObjectiveInterruptedEvent`
  (set `self.TimerEnabled` false)
  (`/Game/Blueprints/BP_FirstPersonCharacter.ObjectiveInterruptedEvent` (`self.PlayerCharacter`)))

(event `ObjectiveCompletedEvent`
  (set `self.TimerEnabled` false)
  (set `self.Timer` (`KismetMathLibrary.Conv_IntToDouble` (`self.TimeLimit`)))
  (set `self.Completed` true)
  (`KismetSystemLibrary.PrintString` "Objective complete")
  (bind _asbp_relay_zero_game_instance (`/Game/Blueprints/FunctionLibraries/BML_Utils.GetGameInstance`))
  (`/Game/FirstPerson/Blueprints/BP_RelayZeroGameInstance.ObjectiveCompletedEvent` _asbp_relay_zero_game_instance))

(fn `CanPlayerSeeObjective`
  (bind (_outhit _returnvalue) (`KismetSystemLibrary.LineTraceSingle` :`Start` (`SceneComponent.K2_GetComponentLocation` (`/Game/Blueprints/BP_FirstPersonCharacter.FirstPersonCamera` (`self.PlayerCharacter`))) :`End` (`SceneComponent.K2_GetComponentLocation` (`self.SM_Computer01`)) :`TraceChannel` "TraceTypeQuery1" :`DrawDebugType` "Persistent"))
  (if _returnvalue
    (if (not (== (`.HitActor` (`GameplayStatics.BreakHitResult` _outhit)) self))
      (`self.ObjectiveInterruptedEvent`))))

(fn `UserConstructionScript`)