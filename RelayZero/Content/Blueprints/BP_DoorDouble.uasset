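; Interactive double door that the player can open, close, lock and unlock by quick interact or an interaction menu that reflects its state.
; Timelines drive mirrored yaw on both leaves, with swing direction chosen from the player's side via a cross product.
; Locking only takes effect when the door is fully closed, and a locked door refuses to open.
; While active, it can show a custom-depth stencil outline.
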(event `/Game/Interfaces/BPI_OutlineGlow.SetOutlineGlow`
  (params (Enabled :type Boolean) (OutlineType :type "/Game/Enums/E_PostProcessingOutlineChannel Enum" :default "NewEnumerator0"))
  (bind _sm_doordouble02_doorl (`self.SM_DoorDouble02_DoorL`))
  ;[1 1 1] Make outline glow
  (if (`self.IsActive`)
    (`PrimitiveComponent.SetRenderCustomDepth` _sm_doordouble02_doorl Enabled)
    (`PrimitiveComponent.SetRenderCustomDepth` (`self.SM_DoorDouble02_DoorR`) Enabled)
    (`PrimitiveComponent.SetRenderCustomDepth` (`self.SM_DoorDouble02_Frame`) Enabled)
    (`PrimitiveComponent.SetCustomDepthStencilValue` _sm_doordouble02_doorl (`KismetMathLibrary.Conv_ByteToInt` OutlineType))
    (`PrimitiveComponent.SetCustomDepthStencilValue` (`self.SM_DoorDouble02_DoorR`) (`KismetMathLibrary.Conv_ByteToInt` OutlineType))
    (`PrimitiveComponent.SetCustomDepthStencilValue` (`self.SM_DoorDouble02_Frame`) (`KismetMathLibrary.Conv_ByteToInt` OutlineType))))

(event `OpenDoorEvent`
  ;[1 0.2648 0.3546] Open, close, lock and unlock
  ;;[1 1 1] Open door
  (`self.CalculateDoorFullyOpenRotation`)
  (if (not (`self.isLocked`))
    (`/Game/Blueprints/FunctionLibraries/BML_Door.IsDoorFullyClosed` (`self.SM_DoorDouble02_DoorR`) (`self.DoorClosedRotation`)
      (:`yes`
        (bind (_direction _alpha) (`Timeline|Timeline_opening` :!via `PlayFromStart` :!label _label)
          (:`Update`
            (`self.Update Door Rotation` _alpha))
          (:`Finished`
            (`self.SetIsOpen` true)
            (`self.UpdateInteractionMenu`))))
      (:`no`
        (goto _label)))))

(event `CloseDoorEvent`
  ;[1 0.2648 0.3546] Open, close, lock and unlock
  ;;[1 1 1] Close door
  (`/Game/Blueprints/FunctionLibraries/BML_Door.IsDoorFullyOpen` (`self.SM_DoorDouble02_DoorR`) (`self.DoorFullyOpenRotation`)
    (:`Yes`
      (bind (_direction _alpha) (`Timeline|Timeline_closing` :!via `ReverseFromEnd` :!label _label_2)
        (:`Update`
          (`self.Update Door Rotation` _alpha))
        (:`Finished`
          (`self.SetIsOpen` false)
          (`self.UpdateInteractionMenu`))))
    (:`No`
      (goto _label_2 :!via `Reverse`))))

(event `LockDoorEvent`
  ;[1 0.2648 0.3546] Open, close, lock and unlock
  ;;[1 1 1] Lock door
  (`self.SetIsLocked` true)
  (`self.UpdateInteractionMenu`))

(event `UnlockDoorEvent`
  ;[1 0.2648 0.3546] Open, close, lock and unlock
  ;;[1 1 1] Unlock door
  (`self.SetIsLocked` false)
  (`self.UpdateInteractionMenu`))

(event `/Game/Interfaces/BPI_Interactable.OnPlayerQuickInteract`
  ;[0.2921 0.3274 1] Player interaction
  ;;[1 1 1] Quick interact
  (if (`self.IsActive`)
    (if (not (`self.isLocked`))
      (`self.ToggleOpenState`))))

(event `/Game/Interfaces/BPI_Interactable.OnPlayerOpenInteractMenu`
  ;[0.2921 0.3274 1] Player interaction
  ;;[1 1 1] Interaction menu
  (`/Game/UI/WeaponWheel/WeaponWheel.OpenMenu` (`self.InteractionMenu`))
  (`self.UpdateInteractionMenu`))

(event `/Game/Interfaces/BPI_Interactable.OnPlayerCloseInteractMenu`
  ;[0.2921 0.3274 1] Player interaction
  ;;[1 1 1] Interaction menu
  (`self.HandleInteractionMenuSelection`)
  (`/Game/UI/WeaponWheel/WeaponWheel.CloseMenu` (`self.InteractionMenu`)))

(fn `CalculateDoorFullyOpenRotation`
  (bind (_returnvalue_x _returnvalue_y _returnvalue_z) (`KismetMathLibrary.BreakVector` (`KismetMathLibrary.Cross_VectorVector` (- (`SceneComponent.K2_GetComponentLocation` (`Character.CapsuleComponent` (`GameplayStatics.GetPlayerCharacter` 0))) (`SceneComponent.K2_GetComponentLocation` (`self.SM_DoorDouble02_Frame`))) (`SceneComponent.GetRightVector` (`self.FrontArrow`)))))
  (if (> _returnvalue_z 0.0)
    ;[1 1 1] Player is to the rear of the door
    (set `self.DoorFullyOpenRotation` (- (`self.DoorClosedRotation`) 90.0))
    (else
      ;[1 1 1] Player is to the front of the door
      (set `self.DoorFullyOpenRotation` (+ (`self.DoorClosedRotation`) 90.0)))))

(fn `HandleInteractionMenuSelection`
  (bind _value (`/Game/UI/WeaponWheel/WeaponWheel.GetSelectedSegmentText` (`self.InteractionMenu`)))
  (switch `string` _value
    (:`Lock`
      (`self.LockDoorEvent`))
    (:`Unlock`
      (`self.UnlockDoorEvent`))
    (:`Open`
      (`self.OpenDoorEvent`))
    (:`Close`
      (`self.CloseDoorEvent`))))

(fn `SetIsLocked`
  (params (NewLockedState :type Boolean))
  (if NewLockedState
    (`/Game/Blueprints/FunctionLibraries/BML_Door.IsDoorFullyClosed` (`self.SM_DoorDouble02_DoorR`) (`self.DoorClosedRotation`)
      (:`yes`
        (set `self.isLocked` true)))
    (else
      (set `self.isLocked` false))))

(fn `SetIsOpen`
  (params (NewIsOpen :type Boolean))
  (if NewIsOpen
    (`self.SetIsLocked` false)
    (set `self.isOpen` true)
    (`SceneComponent.K2_SetRelativeRotation` (`self.SM_DoorDouble02_DoorR`) (`KismetMathLibrary.MakeRotator` 0.0 0.0 (`self.DoorFullyOpenRotation`)) false false)
    (set `self.isOpen` true)
    (`SceneComponent.K2_SetRelativeRotation` (`self.SM_DoorDouble02_DoorL`) (`KismetMathLibrary.MakeRotator` 0.0 0.0 (* (`self.DoorFullyOpenRotation`) -1.0)) false false)
    (else
      (set `self.isOpen` false))))

(fn `ToggleOpenState`
  (if (`self.isOpen`)
    (`self.CloseDoorEvent`)
    (else
      (`self.OpenDoorEvent`))))

(fn `Update Door Rotation`
  (params (alpha :type "Float (double-precision)"))
  (bind _returnvalue (`KismetMathLibrary.Lerp` (`self.DoorClosedRotation`) (`self.DoorFullyOpenRotation`) alpha))
  ;[1 1 1] Doors rotate in opposite directions because relative rotation is flipped based on orientation
  (`SceneComponent.K2_SetRelativeRotation` (`self.SM_DoorDouble02_DoorR`) (`KismetMathLibrary.MakeRotator` 0.0 0.0 _returnvalue) false false)
  (`SceneComponent.K2_SetRelativeRotation` (`self.SM_DoorDouble02_DoorL`) (`KismetMathLibrary.MakeRotator` 0.0 0.0 (* _returnvalue -1.0)) false false))

(fn `UpdateInteractionMenu`
  (if (`self.isOpen`)
    (`/Game/Blueprints/FunctionLibraries/BML_Door.UpdateInteractionMenuDoorOpen` (`self.InteractionMenu`))
    (elif (`self.isLocked`)
      (`/Game/Blueprints/FunctionLibraries/BML_Door.UpdateInteractionMenuDoorLocked` (`self.InteractionMenu`))
      (else
        (`/Game/Blueprints/FunctionLibraries/BML_Door.UpdateInteractionMenuDoorClosed` (`self.InteractionMenu`))))))

(fn `UserConstructionScript`
  (if (`self.isOpen`)
    (`self.SetIsOpen` true)
    (else
      (`self.SetIsOpen` false)
      (`self.SetIsLocked` (`self.isLocked`)))))