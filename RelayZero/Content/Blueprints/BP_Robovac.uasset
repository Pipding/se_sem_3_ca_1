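; Robot vacuum actor that roams on its own, spinning its brushes, and supports outline highlighting through custom depth stencil.
; Each Tick it moves forward without sweep or delta-time scaling until a box trace or capsule overlap flags it blocked.
; When blocked, it randomly tries a 90-degree left or right turn, taken only if that side traces clear.
; Player quick-interact plays a wake chime and reports a noise event.
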(event `ObstacleDetected`
  (params (OverlappedComponent :type "PrimitiveComponent Object Reference") (OtherActor :type "Actor Object Reference") (OtherComp :type "PrimitiveComponent Object Reference") (OtherBodyIndex :type Integer) (bFromSweep :type Boolean) (SweepResult :type "HitResult Structure (by ref)"))
  (set `self.ForwardBlocked` true))

(event `self.ReceiveBeginPlay`
  (`|ExecutionSequence`
    (:`then_0`
      (add `PrimitiveComponent.OnComponentBeginOverlap` (`self.Capsule`) (delegate `ObstacleDetected`)))
    (:`then_1`
      (add `PrimitiveComponent.OnComponentEndOverlap` (`self.Capsule`) (delegate `ObstacleRemoved`)))))

(event `ObstacleRemoved`
  (params (OverlappedComponent :type "PrimitiveComponent Object Reference") (OtherActor :type "Actor Object Reference") (OtherComp :type "PrimitiveComponent Object Reference") (OtherBodyIndex :type Integer))
  (set `self.ForwardBlocked` false))

(event `self.ReceiveTick`
  (params (DeltaSeconds :type "Float (single-precision)"))
  (`self.RotateBrushes` DeltaSeconds)
  (if (`self.ForwardBlocked`)
    (if (`KismetMathLibrary.RandomBool`) :!label _label
      (`self.AttemptRotateLeft`)
      (else
        (`self.AttemptRotateRight`)))
    (else
      (bind _walldetected (`self.DetectWall` "NewEnumerator0"))
      (if _walldetected
        (set `self.ForwardBlocked` true)
        (goto _label)
        (else
          (`self.MoveForward`))))))

(event `/Game/Interfaces/BPI_OutlineGlow.SetOutlineGlow`
  (params (Enabled :type Boolean) (OutlineType :type "/Game/Enums/E_PostProcessingOutlineChannel Enum" :default "NewEnumerator0"))
  (bind _sm_rvc (`self.SM_RVC`))
  ;[1 1 1] TODO: This functionality is duplicated across all implementations. See if it can be defined in the interface
  (`PrimitiveComponent.SetRenderCustomDepth` _sm_rvc Enabled)
  (`PrimitiveComponent.SetCustomDepthStencilValue` _sm_rvc (`KismetMathLibrary.Conv_ByteToInt` OutlineType)))

(event `PlayWakeChimeEvent`
  (bind _returnvalue (`self.K2_GetActorLocation`))
  (`GameplayStatics.PlaySoundAtLocation` "/Game/Assets/Audio/FX/Waves/wake_chime.wake_chime" _returnvalue (struct) 1.0 1.0 0.0 null null null null)
  (`AISense_Hearing.ReportNoiseEvent` _returnvalue 1.0 self 1500.0))

(event `/Game/Interfaces/BPI_Interactable.OnPlayerQuickInteract`
  (`self.PlayWakeChimeEvent`))

(fn `AttemptRotateLeft`
  (bind _walldetected (`self.DetectWall` "NewEnumerator3"))
  (if (not _walldetected)
    (`self.RotateBy` -90.0)
    (set `self.ForwardBlocked` false))
  (return))

(fn `AttemptRotateRight`
  (bind _walldetected (`self.DetectWall` "NewEnumerator1"))
  (if (not _walldetected)
    (`self.RotateBy` 90.0)
    (set `self.ForwardBlocked` false))
  (return))

(fn `DetectWall`
  (params (Direction :type "/Game/Enums/E_Direction Enum" :default "NewEnumerator0"))
  (returns (WallDetected :type Boolean))
  (bind (_start _end) (`self.GetLineTraceVectorsForward`))
  (bind (_start_2 _end_2) (`self.GetLineTraceVectorsRight`))
  (bind (_start_3 _end_3) (`self.GetLineTraceVectorsBack`))
  (bind (_start_4 _end_4) (`self.GetLineTraceVectorsLeft`))
  (bind _relativerotation (`SceneComponent.RelativeRotation` (`self.CollisionCylinder`)))
  (switch `/Game/Enums/E_Direction` Direction
    (:`NewEnumerator0`
      (bind (_outhit _returnvalue) (`KismetSystemLibrary.BoxTraceSingle` _start _end (10.0 30.0 5.0) _relativerotation "TraceTypeQuery1"))
      (return _returnvalue))
    (:`NewEnumerator1`
      (bind (_outhit_2 _returnvalue_2) (`KismetSystemLibrary.BoxTraceSingle` _start_2 _end_2 (10.0 30.0 5.0) _relativerotation "TraceTypeQuery1"))
      (return _returnvalue_2))
    (:`NewEnumerator2`
      (bind (_outhit_3 _returnvalue_3) (`KismetSystemLibrary.BoxTraceSingle` _start_3 _end_3 (10.0 30.0 5.0) _relativerotation "TraceTypeQuery1"))
      (return _returnvalue_3))
    (:`NewEnumerator3`
      (bind (_outhit_4 _returnvalue_4) (`KismetSystemLibrary.BoxTraceSingle` _start_4 _end_4 (10.0 30.0 5.0) _relativerotation "TraceTypeQuery1"))
      (return _returnvalue_4))))

(fn `MoveForward`
  (`self.K2_SetActorLocation` (+ (* (`SceneComponent.GetForwardVector` (`self.CollisionCylinder`)) (`self.Speed`)) (`SceneComponent.K2_GetComponentLocation` (`self.DefaultSceneRoot`)))))

(fn `RotateBrushes`
  (params (DeltaTime :type "Float (double-precision)"))
  (bind _returnvalue (* DeltaTime (`self.BrushRotationSpeed`)))
  (`|ExecutionSequence`
    (:`then_0`
      (`SceneComponent.K2_AddLocalRotation` (`self.SM_RVCBrushLeft`) (`KismetMathLibrary.MakeRotator` 0.0 0.0 _returnvalue) false false))
    (:`then_1`
      (`SceneComponent.K2_AddLocalRotation` (`self.SM_RVCBrushRight`) (`KismetMathLibrary.MakeRotator` 0.0 0.0 _returnvalue) false false))))

(fn `RotateBy`
  (params (angle :type "Float (double-precision)"))
  (bind (_relativerotation_roll _relativerotation_pitch _relativerotation_yaw) (`KismetMathLibrary.BreakRotator` (`SceneComponent.RelativeRotation` (`self.CollisionCylinder`))))
  (`SceneComponent.K2_SetRelativeRotation` (`self.CollisionCylinder`) (`KismetMathLibrary.MakeRotator` _relativerotation_roll _relativerotation_pitch (+ _relativerotation_yaw angle)) false false))

(fn `UserConstructionScript`)