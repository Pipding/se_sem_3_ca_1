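; Interactive lockable door that the player opens, closes, locks or unlocks through a weapon-wheel style menu, or toggles with quick interact.
; Menu selections fire events that update open/locked state and refresh the menu, while timelines rotate the mesh.
; A cross product picks the swing direction from the player's side.
; An attached MetaSound, spawned at BeginPlay to make triggers work, plays door audio, and custom depth stencil drives outline glow.
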(event `self.ReceiveBeginPlay`
  (bind _returnvalue (`|CreateWidget` "/Game/UI/WeaponWheel/WeaponWheel.WeaponWheel_C"))
  (set `self.InteractionMenu` _returnvalue)
  ;[1 1 1] For some unknowable reason, custom triggers only work if we spawn the metasound and attach it manually
  (bind _returnvalue_2 (`GameplayStatics.SpawnSoundAttached` "/Game/Assets/Audio/FX/MS_DoorLock.MS_DoorLock" (`self.SM_Door`) "None" (0.0 0.0 0.0) (struct) "KeepRelativeOffset" false 1.0 1.0 0.0 null null))
  (bind _output_get (set `self.MS_Lock` _returnvalue_2))
  (set `AudioComponent.AttenuationSettings` "/Game/Assets/Audio/FX/AttenuationSettings/Attenuation_Generic.Attenuation_Generic" _output_get))

(event `/Game/Interfaces/BPI_Interactable.OnPlayerOpenInteractMenu`
  (`/Game/UI/WeaponWheel/WeaponWheel.OpenMenu` (`self.InteractionMenu`))
  (`self.UpdateInteractionMenu`))

(event `/Game/Interfaces/BPI_Interactable.OnPlayerCloseInteractMenu`
  (`self.HandleInteractionMenuSelection`)
  (`/Game/UI/WeaponWheel/WeaponWheel.CloseMenu` (`self.InteractionMenu`)))

(event `/Game/Interfaces/BPI_Interactable.OnPlayerQuickInteract`
  ;[1 1 1] Player quick interact
  (if (`/Game/UI/WeaponWheel/WeaponWheel.IsOpen` (`self.InteractionMenu`))
    _
    (elif (`self.isLocked`)
      (message `AudioParameterControllerInterface.SetTriggerParameter` (`self.MS_Lock`) "JiggleHandle")
      (else
        (`self.ToggleOpenedState`)))))

(event `CloseDoorEvent`
  ;[1 1 1] Close door
  (`AudioParameterControllerInterface.SetTriggerParameter` (`self.MS_Lock`) "ClosingStart")
  (`/Game/Blueprints/FunctionLibraries/BML_Door.IsDoorFullyOpen` (`self.SM_Door`) (`self.DoorFullyOpenRotation`)
    (:`Yes`
      (bind (_direction _alpha) (`Timeline|Timeline_closing` :!via `ReverseFromEnd` :!label _label)
        (:`Update`
          (`self.UpdateDoorRotation` _alpha))
        (:`Finished`
          (`self.SetIsOpen` false)
          (`self.UpdateInteractionMenu`)
          (`AudioParameterControllerInterface.SetTriggerParameter` (`self.MS_Lock`) "ClosingEnd"))))
    (:`No`
      (goto _label :!via `Reverse`))))

(event `OpenDoorEvent`
  ;[1 1 1] Open door
  (`self.CalculateDoorFullyOpenRotation`)
  (if (not (`self.isLocked`))
    (`AudioParameterControllerInterface.SetTriggerParameter` (`self.MS_Lock`) "ClosingStart")
    (`/Game/Blueprints/FunctionLibraries/BML_Door.IsDoorFullyClosed` (`self.SM_Door`) (`self.DoorClosedRotation`)
      (:`yes`
        (bind (_direction _alpha) (`Timeline|Timeline_opening` :!via `PlayFromStart` :!label _label_2)
          (:`Update`
            (`self.UpdateDoorRotation` _alpha))
          (:`Finished`
            (`self.SetIsOpen` true)
            (`self.UpdateInteractionMenu`))))
      (:`no`
        (goto _label_2)))))

(event `LockDoorEvent`
  (`AudioParameterControllerInterface.SetTriggerParameter` (`self.MS_Lock`) "Unlock")
  (`self.SetIsLocked` true)
  (`self.UpdateInteractionMenu`))

(event `UnlockDoorEvent`
  (`AudioParameterControllerInterface.SetTriggerParameter` (`self.MS_Lock`) "Unlock")
  (`self.SetIsLocked` false)
  (`self.UpdateInteractionMenu`))

(event `/Game/Interfaces/BPI_OutlineGlow.SetOutlineGlow`
  (params (Enabled :type Boolean) (OutlineType :type "/Game/Enums/E_PostProcessingOutlineChannel Enum" :default "NewEnumerator0"))
  (bind _sm_door (`self.SM_Door`))
  (`PrimitiveComponent.SetRenderCustomDepth` _sm_door Enabled)
  (`PrimitiveComponent.SetRenderCustomDepth` (`self.SM_DoorFrame`) Enabled)
  (`PrimitiveComponent.SetCustomDepthStencilValue` _sm_door (`KismetMathLibrary.Conv_ByteToInt` OutlineType))
  (`PrimitiveComponent.SetCustomDepthStencilValue` (`self.SM_DoorFrame`) (`KismetMathLibrary.Conv_ByteToInt` OutlineType)))

(event `TestEvent_CloseDoor`
  (`SceneComponent.K2_SetRelativeRotation` (`self.SM_Door`) (`KismetMathLibrary.MakeRotator` 0.0 0.0 (`self.DoorClosedRotation`)) false false)
  (`self.CloseDoorEvent`))

(event `TestEvent_SetIsClosed`)

(event `TestEvent_SetIsLocked`)

(fn `CalculateDoorFullyOpenRotation`
  (bind (_returnvalue_x _returnvalue_y _returnvalue_z) (`KismetMathLibrary.BreakVector` (`KismetMathLibrary.Cross_VectorVector` (- (`SceneComponent.K2_GetComponentLocation` (`Character.CapsuleComponent` (`GameplayStatics.GetPlayerCharacter` 0))) (`SceneComponent.K2_GetComponentLocation` (`self.SM_Door`))) (`SceneComponent.GetRightVector` (`self.FrontArrow`)))))
  (if (> _returnvalue_z 0.0)
    (set `self.DoorFullyOpenRotation` (- (`self.DoorClosedRotation`) 90.0))
    (else
      (set `self.DoorFullyOpenRotation` (+ (`self.DoorClosedRotation`) 90.0)))))

(fn `GetIsLocked`
  (returns (isDoorLocked :type Boolean))
  (return (`self.isLocked`)))

(fn `GetIsOpen`
  (returns (isOpen :type Boolean))
  (return (`self.isOpen`)))

(fn `HandleInteractionMenuSelection`
  (bind _value (`/Game/UI/WeaponWheel/WeaponWheel.GetSelectedSegmentText` (`self.InteractionMenu`)))
  (switch `string` _value
    (:`Lock`
      (`self.LockDoorEvent`))
    (:`Unlock`
      (`self.UnlockDoorEvent`))
    (:`Open`
      (`self.OpenDoorEvent`))
    (:`Close`
      (`self.CloseDoorEvent`))))

(fn `SetIsLocked`
  (params (newLockedState :type Boolean))
  (if newLockedState
    (`/Game/Blueprints/FunctionLibraries/BML_Door.IsDoorFullyClosed` (`self.SM_Door`) (`self.DoorClosedRotation`)
      (:`yes`
        (set `self.isLocked` true)))
    (else
      (set `self.isLocked` false))))

(fn `SetIsOpen`
  (params (NewOpenState :type Boolean))
  (if NewOpenState
    (`self.SetIsLocked` false)
    (set `self.isOpen` true)
    (`SceneComponent.K2_SetRelativeRotation` (`self.SM_Door`) (`KismetMathLibrary.MakeRotator` 0.0 0.0 (`self.DoorFullyOpenRotation`)) false false)
    (else
      (set `self.isOpen` false))))

(fn `ToggleOpenedState`
  (`/Game/Blueprints/FunctionLibraries/BML_Door.IsDoorFullyOpen` (`self.SM_Door`) (`self.DoorFullyOpenRotation`)
    (:`Yes`
      _)
    (:`No`
      (`/Game/Blueprints/FunctionLibraries/BML_Door.IsDoorFullyClosed` (`self.SM_Door`) (`self.DoorClosedRotation`)
        (:`yes`
          _))))
  (if (`self.isOpen`)
    (`self.CloseDoorEvent`)
    (else
      (`self.OpenDoorEvent`))))

(fn `UpdateDoorRotation`
  (params (Alpha :type "Float (double-precision)"))
  (`SceneComponent.K2_SetRelativeRotation` (`self.SM_Door`) (`KismetMathLibrary.MakeRotator` 0.0 0.0 (`KismetMathLibrary.Lerp` (`self.DoorClosedRotation`) (`self.DoorFullyOpenRotation`) Alpha)) false false))

(fn `UpdateInteractionMenu`
  (if (`self.isOpen`)
    (`/Game/Blueprints/FunctionLibraries/BML_Door.UpdateInteractionMenuDoorOpen` (`self.InteractionMenu`))
    (elif (`self.isLocked`)
      (`/Game/Blueprints/FunctionLibraries/BML_Door.UpdateInteractionMenuDoorLocked` (`self.InteractionMenu`))
      (else
        (`/Game/Blueprints/FunctionLibraries/BML_Door.UpdateInteractionMenuDoorClosed` (`self.InteractionMenu`))))))

(fn `UserConstructionScript`
  (`StaticMeshComponent.SetStaticMesh` (`self.SM_Door`) (`self.DoorMesh`))
  (if (`self.isOpen`)
    (`self.SetIsOpen` true)
    (else
      (`self.SetIsOpen` false)
      (`self.SetIsLocked` (`self.isLocked`)))))